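; PiggyCharacter is the player character Blueprint, handling jumping, pausing and its startup audio.
; BeginPlay sets game-only input and plays the running sound cue.
; Any non-zero Jump axis value calls Jump and plays the jump sound on each such axis event.
; Pressing P pauses the game, adds a new PauseMenuGUI widget to the viewport and shows the mouse cursor.
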(event EventBeginPlay
  (Input|SetInputModeGameOnly (Game|GetPlayerController 0))
  (Audio|PlaySound2D "/Game/Sounds/Running_Cue.Running_Cue" 1.0 1.0 0.0 0 0))

(event Input|AxisEvents|InputAxisJump
  (params (AxisValue :type Float%20%28single-precision%29))
  (if (not (Math|Float|NearlyEqual(Float) AxisValue 0.0 1e-06))
    (Character|Jump)
    (Audio|PlaySound2D "/Game/Sounds/Jump.Jump" 1.0 1.0 0.0 0 0)))

(event Input|KeyboardEvents|P
  (params (Key :type Key%20Structure))
  (:Pressed
    (Game|SetGamePaused true)
    (bind _returnvalue (UserInterface|CreateWidget "/Game/Blueprints/GUIs/PauseMenuGUI.PauseMenuGUI_C"))
    (UserInterface|Viewport|AddtoViewport _returnvalue 0)
    (Variables|/Script/Engine.PlayerController|SetbShowMouseCursor (Game|GetPlayerController 0) true)))

(fn ConstructionScript)