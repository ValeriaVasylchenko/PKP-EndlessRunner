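; Pumpkin collectable that drifts by a Speed offset every tick and recycles itself instead of being destroyed.
; Overlap with the player broadcasts its Value through an event dispatcher, then resets it; the respawn trigger only resets it, both identified by object name.
; Resetting restores initial X/Y, randomizes height and scale, and derives Value from the rounded scale.
; A DoOnce with a short delay debounces repeat overlaps.
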(event Collision|EventActorBeginOverlap
  (params (OtherActor :type Actor%20Object%20Reference))
  (bind _returnvalue (Utilities|GetObjectName OtherActor))
  (Utilities|FlowControl|DoOnce false :!label _label
    (:Completed
      (if (Utilities|Enum|Equal(Enum) _returnvalue (Utilities|GetObjectName (Game|GetPlayerCharacter 0)))
        (Default|CallPumpkinCollectableED (Variables|Default|GetValue))
        (CallFunction|ResetPosition :!label _label_2)
        (CallFunction|ResetScale)
        (CallFunction|ResetValue)
        (Utilities|FlowControl|Delay 0.2)
        (goto _label Reset)
        (elif (Utilities|Enum|Equal(Enum) _returnvalue (Variables|Default|GetRespawnTriggerName))
          (goto _label_2))))))

(event EventTick
  (params (DeltaSeconds :type Float%20%28single-precision%29))
  (Transformation|AddActorWorldOffset (Variables|Default|GetSpeed)))

(fn ConstructionScript)

(fn ResetPosition
  (bind _initialposition (Variables|Default|GetInitialPosition))
  (bind (_x _y) (Math|Vector|BreakVector _initialposition))
  (Transformation|SetActorLocation (Math|Vector|MakeVector _x _y (Math|Random|RandomFloatinRange 1.4e+02 4e+02)) false false))

(fn ResetScale
  (bind _output_get (Variables|Default|SetScale (Math|Random|RandomFloatinRange 1.0 5.0)))
  (Transformation|SetActorScale3D (Math|Vector|MakeVector (/ _output_get 1e+01) (/ _output_get 1e+01) (/ _output_get 1e+01))))

(fn ResetValue
  (Variables|Default|SetValue (Math|Float|Round (Variables|Default|GetScale))))